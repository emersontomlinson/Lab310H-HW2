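; BP_Target is a shootable target actor that drives level progression in a first-person game.
; Each hit from a BP_FirstPersonProjectile lowers its Health, and at zero it increments the player character's TargetsHit counter.
; Once that count reaches three it opens Level2 from Level1, or MainMenu from any other level; otherwise the target destroys itself.
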(event `self.ReceiveHit`
  (params (MyComp :type "PrimitiveComponent Object Reference") (Other :type "Actor Object Reference") (OtherComp :type "PrimitiveComponent Object Reference") (bSelfMoved :type Boolean) (HitLocation :type "Vector Structure") (HitNormal :type "Vector Structure") (NormalImpulse :type "Vector Structure") (Hit :type "HitResult Structure (by ref)"))
  (cast `/Game/FirstPerson/Blueprints/BP_FirstPersonProjectile` Other)
  (bind _output_get (set `self.Health` (- (`self.Health`) 25)))
  (if (<= _output_get 0)
    (bind _asbp_first_person_character (cast `/Game/FirstPerson/Blueprints/BP_FirstPersonCharacter` (`GameplayStatics.GetPlayerCharacter` 0)))
    (bind _output_get_2 (set `/Game/FirstPerson/Blueprints/BP_FirstPersonCharacter.TargetsHit` (+ (`/Game/FirstPerson/Blueprints/BP_FirstPersonCharacter.TargetsHit` _asbp_first_person_character) 1) _asbp_first_person_character))
    (if (>= _output_get_2 3)
      (bind _returnvalue (`GameplayStatics.GetCurrentLevelName` true))
      (if (`KismetStringLibrary.EqualEqual_StrStr` _returnvalue "Level1")
        (`GameplayStatics.OpenLevel` "Level2")
        (else
          (`GameplayStatics.OpenLevel` "MainMenu")))
      (else
        (`self.K2_DestroyActor`)))))

(fn `UserConstructionScript`)